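; BP_Human is an enemy character that chases the player and punches them.
; From BeginPlay and on pawn sighting, AIMoveTo closes in, then plays a punch montage gated by a DoOnce.
; A toggleable Sphere collider deals damage and plays a punch sound when it overlaps the player.
; Any damage kills it once: it ragdolls away from the damage causer with blood and pain sound, then is destroyed after a delay.
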(event `self.ReceiveAnyDamage`
  (params (Damage :type "Float (single-precision)") (DamageType :type "DamageType Object Reference") (InstigatedBy :type "Controller Object Reference") (DamageCauser :type "Actor Object Reference"))
  (bind _mesh (`self.Mesh`))
  ; death
  (`/Engine/EditorBlueprintResources/StandardMacros.DoOnce` false
    (:`Completed`
      (`PrimitiveComponent.SetCollisionProfileName` _mesh "Ragdoll" true)
      (`PrimitiveComponent.SetCollisionResponseToChannel` _mesh "ECC_Pawn" "ECR_Ignore")
      (`PrimitiveComponent.SetSimulatePhysics` _mesh true)
      (`PrimitiveComponent.SetCollisionResponseToChannel` (`self.CapsuleComponent`) "ECC_Pawn" "ECR_Ignore")
      (`PrimitiveComponent.SetCollisionResponseToChannel` (`self.Mesh`) "ECC_Camera" "ECR_Ignore")
      (`PrimitiveComponent.SetCollisionResponseToChannel` (`self.CapsuleComponent`) "ECC_Camera" "ECR_Ignore")
      (`PrimitiveComponent.SetPhysicsLinearVelocity` (`self.Mesh`) (* (`KismetMathLibrary.Normal` (- (`self.K2_GetActorLocation`) (`self.K2_GetActorLocation` DamageCauser))) 9000.0) true "None")
      ;; disable animations when dead
      (`SkeletalMeshComponent.SetAnimInstanceClass` (`self.Mesh`) null)
      (`ActorComponent.Activate` (`self.NS_BloodFX`) false)
      (`GameplayStatics.PlaySoundAtLocation` "/Game/SFX/Humangrunts/SC_HumanPain.SC_HumanPain" (`self.K2_GetActorLocation`) (struct) 1.0 1.0 0.0 null null null null)
      (`KismetSystemLibrary.Delay` 40.0)
      (`self.K2_DestroyActor`))))

(event `self.PawnSensing.OnSeePawn`
  (params (Pawn :type "Pawn Object Reference"))
  ; chase player and punch
  (`|AIMoveTo` self (0.0 0.0 0.0) (`GameplayStatics.GetPlayerCharacter` 0) 15.0 :!label _label
    (:`OnSuccess`
      (`/Engine/EditorBlueprintResources/StandardMacros.DoOnce` false :!label _label_2
        (:`Completed`
          (`|PlayMontage` (`self.Mesh`) "/Game/Man/Demo/Animations/A_Manpunch_Montage.A_Manpunch_Montage"
            (:`OnCompleted`
              (goto _label_2 :!via `Reset`))
            (:`OnInterrupted`
              (goto _label_2 :!via `Reset`))))))))

(event `Toggle Human Collision`
  (params (`true?` :type Boolean))
  (bind _sphere (`self.Sphere`))
  ; toggle punch collision
  (if `true?`
    (`PrimitiveComponent.SetCollisionEnabled` _sphere "QueryAndPhysics")
    (else
      (`PrimitiveComponent.SetCollisionEnabled` _sphere "NoCollision"))))

(event `self.Sphere.OnComponentBeginOverlap`
  (params (OverlappedComponent :type "PrimitiveComponent Object Reference") (OtherActor :type "Actor Object Reference") (OtherComp :type "PrimitiveComponent Object Reference") (OtherBodyIndex :type Integer) (bFromSweep :type Boolean) (SweepResult :type "HitResult Structure (by ref)"))
  (bind _returnvalue (`GameplayStatics.GetPlayerCharacter` 0))
  ; apply damage to the player
  (if (== OtherActor _returnvalue)
    (`GameplayStatics.ApplyDamage` _returnvalue 2.0)
    (`GameplayStatics.PlaySoundAtLocation` "/Game/SFX/Human_punch/qubodupPunch02.qubodupPunch02" (`self.K2_GetActorLocation`) (struct) 1.0 1.0 0.0 null null null null)))

(event `self.ReceiveBeginPlay`
  (`PrimitiveComponent.SetCollisionEnabled` (`self.Sphere`) "NoCollision")
  (goto _label))

(fn `UserConstructionScript`)