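; BP_HealthPickup is a health pickup that heals the player's gorilla on contact and then destroys itself.
; A Box overlap checks that the overlapping actor is the player pawn cast to BP_Gorilla, then calls Heal with HealingAmount.
; On BeginPlay it registers with the LevelManager, if valid, so a level reset event also destroys the pickup.
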(event `self.ReceiveBeginPlay`
  (bind _levelmanager (`self.LevelManager`)
    (:`then`
      (add `/Game/Blueprints/BP_LevelManager.LevelReset` _levelmanager (delegate `LevelReset_Event`)))
    (:`else`)))

(event `LevelReset_Event`
  (`self.K2_DestroyActor`))

(event `self.Box.OnComponentBeginOverlap`
  (params (OverlappedComponent :type "PrimitiveComponent Object Reference") (OtherActor :type "Actor Object Reference") (OtherComp :type "PrimitiveComponent Object Reference") (OtherBodyIndex :type Integer) (bFromSweep :type Boolean) (SweepResult :type "HitResult Structure (by ref)"))
  (bind _asbp_gorilla (cast `/Game/Blueprints/BP_Gorilla` (`GameplayStatics.GetPlayerPawn` 0)))
  (if (== OtherActor _asbp_gorilla)
    (`/Game/Blueprints/BP_Gorilla.Heal` _asbp_gorilla (`self.HealingAmount`))
    (`self.K2_DestroyActor`)))

(fn `UserConstructionScript`)