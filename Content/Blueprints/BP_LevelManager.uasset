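; BP_LevelManager runs the wave-based levels in a game where the player's gorilla faces humans, managing timer and human-counter widgets.
; SetUpLevel spawns growing crowds of BP_Human at random reachable points across four waves, then just stops the timer.
; When no humans remain, NextLevel shows the next wave, pauses, heals the gorilla and calls a level reset before spawning.
; A DoOnce-and-delay loop on Tick periodically spawns health pickups.
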(event `self.ReceiveBeginPlay`
  (bind _timerwidgetref (`self.timerWidgetRef`))
  (bind _asbp_gorilla (cast `/Game/Blueprints/BP_Gorilla` (`GameplayStatics.GetPlayerPawn` 0)))
  (bind _output_get (set `self.playerGorillaRef` _asbp_gorilla))
  (set `self.gorillaOrigTransform` (`self.GetTransform` _output_get))
  (set `self.currentLevel` 0)
  ; create and add to viewport the Timer and Human Counter widgets
  (bind _returnvalue (`|CreateWidget` "/Game/Widgets/WB_Timer.WB_Timer_C"))
  (bind _output_get_2 (set `self.timerWidgetRef` _returnvalue))
  (`UserWidget.AddToViewport` _output_get_2 0)
  (bind _returnvalue_2 (`|CreateWidget` "/Game/Widgets/WB_Humans.WB_Humans_C"))
  (bind _output_get_3 (set `self.humanWidgetRef` _returnvalue_2))
  (`UserWidget.AddToViewport` _output_get_3 0)
  (`/Game/Widgets/WB_Timer.NextWave` _timerwidgetref 0)
  (`KismetSystemLibrary.Delay` 5.0)
  (`/Game/Widgets/WB_Timer. RestartTimer` _timerwidgetref)
  (`self.LevelReset`)
  (`self.SetUpLevel` (`self.currentLevel`))
  (`/Game/Widgets/WB_Timer.StopWave` _timerwidgetref))

(event `NextLevel`
  (bind _currentlevel (`self.currentLevel`))
  (bind _timerwidgetref (`self.timerWidgetRef`))
  ; check if all enemies are dead and, if so, start up the next level (should have made this a function)
  (if (<= (`self.humans`) 0)
    (`/Engine/EditorBlueprintResources/StandardMacros.IncrementInt` _currentlevel
      (:`  `
        (`/Game/Widgets/WB_Timer.StopTimer` _timerwidgetref)
        (`/Game/Widgets/WB_Timer.NextWave` _timerwidgetref _currentlevel)
        (`KismetSystemLibrary.Delay` 5.0)
        (`/Game/Widgets/WB_Timer. RestartTimer` _timerwidgetref)
        (`/Game/Blueprints/BP_Gorilla.Heal` (`self.playerGorillaRef`) 100.0)
        (`self.LevelReset`)
        (`self.SetUpLevel` _currentlevel)
        (`/Game/Widgets/WB_Timer.StopWave` (`self.timerWidgetRef`))))))

(event `self.ReceiveTick`
  (params (DeltaSeconds :type "Float (single-precision)"))
  ; spawn health item every now and again
  (`/Engine/EditorBlueprintResources/StandardMacros.DoOnce` false :!label _label
    (:`Completed`
      (`self.SpawnHealth`)
      (`KismetSystemLibrary.Delay` (`KismetMathLibrary.RandomFloatInRange` 4.0 6.0))
      (goto _label :!via `Reset`))))

(event `SpawnHealth`
  ; Spawn health item in accesible zone
  (`|SpawnActorFromClass` "/Game/Blueprints/BP_HealthPickup.BP_HealthPickup_C" (`KismetMathLibrary.MakeTransform` (`NavigationSystemV1.K2_GetRandomReachablePointInRadius` (`self.K2_GetActorLocation`) 4000.0 null null)) "Undefined" "MultiplyWithRoot" null self null))

(fn `SetUpLevel`
  (params (LevelNum :type Integer))
  (bind _humanwidgetref (`self.humanWidgetRef`))
  (switch `int` LevelNum
    (:`Default`
      (`/Game/Widgets/WB_Timer.StopTimer` (`self.timerWidgetRef`)))
    (:`0`
      (set `self.spawnAmount` 9)
      (for _ (range (+ (`self.spawnAmount`) 1)) :!label _label
        (`|SpawnActorFromClass` "/Game/Blueprints/BP_Human.BP_Human_C" (`KismetMathLibrary.MakeTransform` (`NavigationSystemV1.K2_GetRandomReachablePointInRadius` (`self.K2_GetActorLocation`) 4000.0 null null)) "AdjustIfPossibleButAlwaysSpawn" "MultiplyWithRoot" null (`self.humanWidgetRef`) self null)
        (`/Engine/EditorBlueprintResources/StandardMacros.IncrementInt` (`self.humans`)))
      (set `/Game/Widgets/WB_Humans.humans` (`self.humans`) _humanwidgetref)
      (`/Game/Widgets/WB_Humans.UpdateHumans` _humanwidgetref))
    (:`1`
      (set `self.spawnAmount` 24)
      (goto _label))
    (:`2`
      (set `self.spawnAmount` 49)
      (goto _label))
    (:`3`
      (set `self.spawnAmount` 99)
      (goto _label))))

(fn `UserConstructionScript`)